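; Client1 is a Socket.IO client Blueprint that creates and joins server-side parties, reporting results through debug prints.
; On connect, it binds a broadcast listener, emits create and a test chat message, then requests the party list.
; Callback-based emits chain the flow: OnGetParties refills Parties and joins the first entry, and ConnectResponse prints the join result.
; GetGames ignores its Callback parameter, reusing OnGetParties.
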(event `self.SocketIOClient.OnComponentActivated`
  (params (Component :type "ActorComponent Object Reference") (bReset :type Boolean))
  (`KismetSystemLibrary.PrintString` "Activated !"))

(event `self.SocketIOClient.OnConnected`
  (params (SocketId :type String) (SessionId :type String) (bIsReconnection :type Boolean))
  (`SocketIOClientComponent.BindEventToDelegate` (`self.SocketIOClient`) "broadcast" (delegate `On Broadcast`) "/" "USE_DEFAULT")
  (`KismetSystemLibrary.PrintString` "connected to the server")
  (`self.Emit` "create")
  (`self.Emit` "chat" "Ping !")
  (`SocketIOClientComponent.EmitWithCallBack` (`self.SocketIOClient`) "get_parties" null "OnGetParties" null "/"))

(event `On Broadcast`
  (params (EventData :type "SIOJsonValue Object Reference"))
  (`KismetSystemLibrary.PrintString` (`SIOJLibrary.Conv_SIOJsonValueToString` EventData)))

(fn `ConnectResponse`
  (params (Message :type "SIOJsonValue Object Reference"))
  (`KismetSystemLibrary.PrintString` (`KismetStringLibrary.Concat_StrStr` "connected : " (`KismetStringLibrary.Conv_BoolToString` (`SIOJLibrary.Conv_JsonValueToBool` Message)))))

(fn `Emit`
  (params (event :type String) (message :type String))
  (`SocketIOClientComponent.Emit` (`self.SocketIOClient`) event (`SIOJLibrary.Conv_StringToJsonValue` message) "/"))

(fn `GetGames`
  (params (Callback :type "Delegate (by ref)"))
  (`SocketIOClientComponent.EmitWithCallBack` (`self.SocketIOClient`) "get_games" null "OnGetParties" null "/"))

(fn `OnGetParties`
  (params (Message :type "SIOJsonValue Object Reference"))
  (`KismetArrayLibrary.Array_Clear` (`self.parties`))
  (for _array_element (`SIOJsonValue.AsArray` Message)
    (bind _returnvalue (`SIOJLibrary.Conv_SIOJsonValueToString` _array_element))
    (`KismetArrayLibrary.Array_Add` (`self.parties`) _returnvalue)
    (`KismetSystemLibrary.PrintString` _returnvalue))
  (`self.TryConnect` (`|GetArrayItem` (`self.parties`))))

(fn `TryConnect`
  (params (id :type String))
  (`SocketIOClientComponent.EmitWithCallBack` (`self.SocketIOClient`) "join" (`SIOJLibrary.Conv_StringToJsonValue` id) "ConnectResponse" null "/"))

(fn `UserConstructionScript`)