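; ClientUser is a test Blueprint that exercises the game's Socket.IO client and prints the results to screen.
; On BeginPlay it caches GenericGameInstance, binds connection and "broadcast" events on its Client, then emits "create" twice, a "chat" PING and "get_games".
; Callbacks print success or a red error through PrintCallback, while the get_games response and broadcast messages are printed directly.
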(event `self.ReceiveBeginPlay`
  (`self.SetGameInstance`)
  (add `SocketIOClientComponent.OnConnected` (`Client.SIOClientComponent` (`/Game/Blueprints/GenericGameInstance.Client` (`self.GameInstance`))) (delegate `CustomEvent_6`))
  (`Client.BindEventTo` (`/Game/Blueprints/GenericGameInstance.Client` (`self.GameInstance`)) "broadcast" (delegate `CustomEvent_5`))
  (`Client.Emit` (`/Game/Blueprints/GenericGameInstance.Client` (`self.GameInstance`)) "create" null (delegate `CustomEvent_1`))
  (`Client.Emit` (`/Game/Blueprints/GenericGameInstance.Client` (`self.GameInstance`)) "create" null (delegate `CustomEvent_2`))
  (`Client.Emit` (`/Game/Blueprints/GenericGameInstance.Client` (`self.GameInstance`)) "chat" (`SIOJLibrary.Conv_StringToJsonValue` "PING") (delegate `CustomEvent_0`))
  (`Client.Emit` (`/Game/Blueprints/GenericGameInstance.Client` (`self.GameInstance`)) "get_games" null (delegate `CustomEvent_4`)))

(event `CustomEvent_6`
  (params (SocketId :type String) (SessionId :type String) (bIsReconnection :type Boolean))
  (`KismetSystemLibrary.PrintString` "Connected !"))

(event `CustomEvent_1`
  (params (callbackStruct :type "CallbackStruct Structure"))
  (`self.PrintCallback` "create" callbackStruct))

(event `CustomEvent_2`
  (params (callbackStruct :type "CallbackStruct Structure"))
  (`self.PrintCallback` "create" callbackStruct))

(event `CustomEvent_0`
  (params (callbackStruct :type "CallbackStruct Structure"))
  (`self.PrintCallback` "chat" callbackStruct))

(event `CustomEvent_4`
  (params (callbackStruct :type "CallbackStruct Structure"))
  (`KismetSystemLibrary.PrintString` (`SIOJLibrary.Conv_SIOJsonValueToString` callbackStruct_data))
  (if callbackStruct_success
    (for _array_element (`SIOJsonValue.AsArray` callbackStruct_data)
      (`KismetSystemLibrary.PrintString` (`SIOJLibrary.Conv_SIOJsonValueToString` _array_element)))))

(event `CustomEvent_5`
  (params (EventData :type "SIOJsonValue Object Reference"))
  (`KismetSystemLibrary.PrintString` (`SIOJsonObject.GetStringField` (`SIOJLibrary.Conv_JsonValueToJsonObject` EventData) "message")))

(fn `PrintCallback`
  (params (RequestName :type String) (Callback :type "CallbackStruct Structure"))
  (if Callback_success
    (`KismetSystemLibrary.PrintString` (`KismetStringLibrary.Concat_StrStr` "SUCCESS : " RequestName))
    (else
      (`KismetSystemLibrary.PrintString` (`KismetStringLibrary.Concat_StrStr` (`KismetStringLibrary.Concat_StrStr` (`KismetStringLibrary.Concat_StrStr` (`KismetStringLibrary.Concat_StrStr` "ERROR : " RequestName) " (") Callback_message) ")") true true (struct :`R` 1.0 :`B` 0.024068 :`A` 1.0)))))

(fn `SetGameInstance`
  (bind _asgeneric_game_instance (cast `/Game/Blueprints/GenericGameInstance` (`GameplayStatics.GetGameInstance`)))
  (set `self.GameInstance` _asgeneric_game_instance))

(fn `UserConstructionScript`)